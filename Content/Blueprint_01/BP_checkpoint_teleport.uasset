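; BP_checkpoint_teleport is a checkpoint actor that records a respawn point on the third-person character when it overlaps.
; On overlap, it writes its own location to the character's CheckpointLocation and tints the mesh's "Paint Tint" material parameter bright green, then pale cream after a one-second delay.
; The teleport itself is not performed here; the Hit event only casts and does nothing further.
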(event EventBeginPlay)

(event EventTick
  (params (DeltaSeconds :type Float%20%28single-precision%29)))

(event Collision|EventActorBeginOverlap
  (params (OtherActor :type Actor%20Object%20Reference))
  (bind _asbp_third_person_character (Utilities|Casting|CastToBP_ThirdPersonCharacter OtherActor))
  (Variables|/Game/ThirdPerson/Blueprints/BP_ThirdPersonCharacter.BP_ThirdPersonCharacter_C|SetCheckpoint_location _asbp_third_person_character (Transformation|GetActorLocation))
  (Rendering|Material|SetColorParameterValueonMaterials (Variables|/Script/Engine.Character|GetMesh _asbp_third_person_character) "Paint Tint" "(R=0.339696,G=1.000000,B=0.000000,A=1.000000)")
  (Utilities|FlowControl|Delay 1.0)
  (Rendering|Material|SetColorParameterValueonMaterials (Variables|/Script/Engine.Character|GetMesh _asbp_third_person_character) "Paint Tint" "(R=0.958151,G=1.000000,B=0.832261,A=1.000000)"))

(event Collision|EventHit
  (params (MyComp :type Primitive%20Component%20Object%20Reference) (Other :type Actor%20Object%20Reference) (OtherComp :type Primitive%20Component%20Object%20Reference) (bSelfMoved :type Boolean) (HitLocation :type Vector :default "0, 0, 0") (HitNormal :type Vector :default "0, 0, 0") (NormalImpulse :type Vector :default "0, 0, 0") (Hit :type Hit%20Result%20Structure%20%28by%20ref%29))
  (Utilities|Casting|CastToBP_ThirdPersonCharacter Other))

(fn ConstructionScript)